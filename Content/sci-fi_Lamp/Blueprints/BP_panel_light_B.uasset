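; BP_panel_light_B is a sci-fi panel lamp that pairs a mesh with a dynamic short-range rect light.
; Its construction script pushes the exposed color, intensity, radius, temperature, scattering, indirect lighting, barn door and shadow settings onto the light.
; It also creates a dynamic material instance on the mesh from EmissiveMaterial, without setting any parameters on it.
; A parallel GI light setup is left unconnected, and the event graph is empty.
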(event EventBeginPlay)

(event Collision|EventActorBeginOverlap
  (params (OtherActor :type Actor%20Object%20Reference)))

(event EventTick
  (params (DeltaSeconds :type Float%20%28single-precision%29)))

(fn ConstructionScript
  (bind _lit_rectlight_dynamic_shortrange_a01 (Variables|Default|GetLit_RectLight_Dynamic_Shortrange_A01))
  (Utilities|FlowControl|Sequence
    (:then_0
      ;[1 1 1] Dynamic
      (Rendering|Components|Light|SetLightColor _lit_rectlight_dynamic_shortrange_a01 (Variables|DynamicLight|GetLight%20Color) true)
      (Rendering|Components|Light|SetIntensity _lit_rectlight_dynamic_shortrange_a01 (Variables|DynamicLight|GetIntensity%20%28Dynamic%29))
      (Rendering|Lighting|SetAttenuationRadius _lit_rectlight_dynamic_shortrange_a01 (Variables|DynamicLight|GetRadius%20%28Dynamic%29))
      (Rendering|Material|CreateDynamicMaterialInstance (Variables|Default|GetSM_panel_light_B) 0 (Variables|DynamicLight|GetEmissive%20Material) "None" :!class /Script/Engine.PrimitiveComponent)
      (Class|LightComponent|SetVolumetricScatteringIntensity _lit_rectlight_dynamic_shortrange_a01 (Variables|DynamicLight|GetVolumetric%20scattering%20Intensity%20%28Dynamic%29))
      (Class|LightComponent|SetIndirectLightingIntensity _lit_rectlight_dynamic_shortrange_a01 (Variables|DynamicLight|GetIndirect%20Lighting%20Intensity%20%28Dynamic%29))
      (Class|RectLightComponent|SetBarnDoorAngle _lit_rectlight_dynamic_shortrange_a01 (Variables|DynamicLight|GetBarn%20Door%20Angle%20%28Dynamic%29))
      (Rendering|Components|Light|SetCastShadows _lit_rectlight_dynamic_shortrange_a01 (Variables|DynamicLight|GetCast%20Shadow%20%28Dynamic%29))
      (Class|LightComponent|SetTemperature _lit_rectlight_dynamic_shortrange_a01 (Variables|DynamicLight|GetTemperature)))))