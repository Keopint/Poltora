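; Pendant lamp prop Blueprint for a sci-fi lamp set, configurable per instance through exposed light and material variables.
; The Construction Script pushes shared cone, color, intensity, radius, shadow and temperature settings onto three short-range dynamic spotlights.
; A separate GI spotlight takes its own GI values but shares color and temperature, and the mesh gets a dynamic emissive material instance.
; The event graph holds no active logic.
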(event EventBeginPlay)

(event Collision|EventActorBeginOverlap
  (params (OtherActor :type Actor%20Object%20Reference)))

(event EventTick
  (params (DeltaSeconds :type Float%20%28single-precision%29)))

(fn ConstructionScript
  (bind _lit_spotlight_gi_01a (Variables|Default|GetLIT_SpotLight_GI_01A))
  (bind _lit_spotlight_dynamic_shortrange_02a (Variables|Default|GetLIT_SpotLight_Dynamic_ShortRange_02A))
  (bind _lit_spotlight_dynamic_shortrange_03a (Variables|Default|GetLIT_SpotLight_Dynamic_ShortRange_03A))
  (bind _lit_spotlight_dynamic_shortrange_01a (Variables|Default|GetLIT_SpotLight_Dynamic_ShortRange_01A))
  (Utilities|FlowControl|Sequence
    (:then_0
      ;[1 1 1] Dynamic Light
      (Rendering|Lighting|SetInnerConeAngle _lit_spotlight_dynamic_shortrange_01a (Variables|SpotLight_Dynamic|GetInner%20Cone%20Angle))
      (Rendering|Lighting|SetOuterConeAngle _lit_spotlight_dynamic_shortrange_01a (Variables|SpotLight_Dynamic|GetOuter%20Cone%20Angle))
      (Rendering|Components|Light|SetLightColor _lit_spotlight_dynamic_shortrange_01a (Variables|SpotLight_Dynamic|GetDynamic%20Light%20Color) true)
      (Rendering|Components|Light|SetIntensity _lit_spotlight_dynamic_shortrange_01a (Variables|SpotLight_Dynamic|GetIntensity))
      (Rendering|Lighting|SetAttenuationRadius _lit_spotlight_dynamic_shortrange_01a (Variables|SpotLight_Dynamic|GetRadius))
      (Rendering|Material|CreateDynamicMaterialInstance (Variables|Default|GetSM_pendant_Lamp_C) 1 (Variables|SpotLight_Dynamic|GetEmissive%20Material) "None" :!class /Script/Engine.PrimitiveComponent)
      (Class|LightComponent|SetVolumetricScatteringIntensity _lit_spotlight_dynamic_shortrange_01a (Variables|SpotLight_Dynamic|GetVolumetric%20scattering%20Intensity))
      (Class|LightComponent|SetIndirectLightingIntensity _lit_spotlight_dynamic_shortrange_01a (Variables|SpotLight_Dynamic|GetIndirect%20Lighting%20Intensity))
      (Rendering|Components|Light|SetCastShadows _lit_spotlight_dynamic_shortrange_01a (Variables|SpotLight_Dynamic|GetCast%20Shadow))
      (Class|LightComponent|SetTemperature _lit_spotlight_dynamic_shortrange_01a (Variables|SpotLight_Dynamic|GetTemperature)))
    (:then_1
      (Rendering|Lighting|SetInnerConeAngle _lit_spotlight_dynamic_shortrange_02a (Variables|SpotLight_Dynamic|GetInner%20Cone%20Angle))
      (Rendering|Lighting|SetOuterConeAngle _lit_spotlight_dynamic_shortrange_02a (Variables|SpotLight_Dynamic|GetOuter%20Cone%20Angle))
      (Rendering|Components|Light|SetLightColor _lit_spotlight_dynamic_shortrange_02a (Variables|SpotLight_Dynamic|GetDynamic%20Light%20Color) true)
      (Rendering|Components|Light|SetIntensity _lit_spotlight_dynamic_shortrange_02a (Variables|SpotLight_Dynamic|GetIntensity))
      (Rendering|Lighting|SetAttenuationRadius _lit_spotlight_dynamic_shortrange_02a (Variables|SpotLight_Dynamic|GetRadius))
      (Class|LightComponent|SetVolumetricScatteringIntensity _lit_spotlight_dynamic_shortrange_02a (Variables|SpotLight_Dynamic|GetVolumetric%20scattering%20Intensity))
      (Class|LightComponent|SetIndirectLightingIntensity _lit_spotlight_dynamic_shortrange_02a (Variables|SpotLight_Dynamic|GetIndirect%20Lighting%20Intensity))
      (Rendering|Components|Light|SetCastShadows _lit_spotlight_dynamic_shortrange_02a (Variables|SpotLight_Dynamic|GetCast%20Shadow))
      (Class|LightComponent|SetTemperature _lit_spotlight_dynamic_shortrange_02a (Variables|SpotLight_Dynamic|GetTemperature)))
    (:then_2
      (Rendering|Lighting|SetInnerConeAngle _lit_spotlight_dynamic_shortrange_03a (Variables|SpotLight_Dynamic|GetInner%20Cone%20Angle))
      (Rendering|Lighting|SetOuterConeAngle _lit_spotlight_dynamic_shortrange_03a (Variables|SpotLight_Dynamic|GetOuter%20Cone%20Angle))
      (Rendering|Components|Light|SetLightColor _lit_spotlight_dynamic_shortrange_03a (Variables|SpotLight_Dynamic|GetDynamic%20Light%20Color) true)
      (Rendering|Components|Light|SetIntensity _lit_spotlight_dynamic_shortrange_03a (Variables|SpotLight_Dynamic|GetIntensity))
      (Rendering|Lighting|SetAttenuationRadius _lit_spotlight_dynamic_shortrange_03a (Variables|SpotLight_Dynamic|GetRadius))
      (Class|LightComponent|SetVolumetricScatteringIntensity _lit_spotlight_dynamic_shortrange_03a (Variables|SpotLight_Dynamic|GetVolumetric%20scattering%20Intensity))
      (Class|LightComponent|SetIndirectLightingIntensity _lit_spotlight_dynamic_shortrange_03a (Variables|SpotLight_Dynamic|GetIndirect%20Lighting%20Intensity))
      (Rendering|Components|Light|SetCastShadows _lit_spotlight_dynamic_shortrange_03a (Variables|SpotLight_Dynamic|GetCast%20Shadow))
      (Class|LightComponent|SetTemperature _lit_spotlight_dynamic_shortrange_03a (Variables|SpotLight_Dynamic|GetTemperature)))
    (:then_3
      ;[1 1 1] GI Light
      (Rendering|Lighting|SetInnerConeAngle _lit_spotlight_gi_01a (Variables|GILight|GetInner%20Cone%20Angle%28GI%29))
      (Rendering|Lighting|SetOuterConeAngle _lit_spotlight_gi_01a (Variables|GILight|GetOuter%20Cone%20Angle%28GI%29))
      (Rendering|Components|Light|SetLightColor _lit_spotlight_gi_01a (Variables|SpotLight_Dynamic|GetDynamic%20Light%20Color) true)
      (Rendering|Components|Light|SetIntensity _lit_spotlight_gi_01a (Variables|GILight|GetIntensity%20%28GI%29))
      (Rendering|Lighting|SetAttenuationRadius _lit_spotlight_gi_01a (Variables|GILight|GetRadius%20%28GI%29))
      (Class|LightComponent|SetIndirectLightingIntensity _lit_spotlight_gi_01a (Variables|GILight|GetIndirect%20Lighting%20Intensity%20%28GI%29))
      (Rendering|Components|Light|SetCastShadows _lit_spotlight_gi_01a (Variables|GILight|GetCast%20Shadow%20%28GI%29))
      (Class|LightComponent|SetTemperature _lit_spotlight_gi_01a (Variables|SpotLight_Dynamic|GetTemperature)))))