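; Moving platform with a turret head that fires at sensed pawns tagged Enemy.
; The construction script gives InterpToMovement a path from the actor's origin to MoveToPos.
; On sighting, the head turns toward the pawn with clamped pitch and runs a looping Fire timer for a short burst.
; Fire traces forward and spawns a scaled-down TurretBullet only when the hit actor lacks the Enemy tag.
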(event OnSeePawn(PawnSensing)
  (params (Pawn :type Pawn%20Object%20Reference))
  (bind _returnvalue (Transformation|GetActorLocation Pawn))
  (bind _turrethead (Variables|Default|GetturretHead))
  (bind _returnvalue_2 (Transformation|GetWorldLocation _turrethead))
  (bind _returnvalue_3 (- _returnvalue "0.000000,0.000000,100.000000"))
  (bind _returnvalue_4 (Math|Rotator|FindLookatRotation _returnvalue_2 _returnvalue_3))
  (bind (_roll _pitch _yaw) (Math|Rotator|BreakRotator _returnvalue_4))
  (if (> (Transformation|GetDistanceTo Pawn (Components|GetOwner (Variables|Default|GetturretHead))) 0.0)
    (if (Actor|ActorHasTag Pawn "Enemy")
      (Transformation|SetWorldRotation (Variables|Default|GetturretHead) (Math|Rotator|MakeRotator _roll (Math|Float|Clamp(Float) _pitch -2e+01 2e+01) _yaw) false false)
      (bind _returnvalue_5 (Utilities|Time|SetTimerbyEvent (delegate Custom|Fire) 0.1 true))
      (Utilities|FlowControl|Delay 1.0)
      (Utilities|Time|ClearandInvalidateTimerbyHandle _returnvalue_5))))

(event Custom|Fire
  (bind _turrethead (Variables|Default|GetturretHead))
  (bind _turrethead_2 (Variables|Default|GetturretHead))
  (bind _returnvalue (Transformation|GetWorldTransform _turrethead))
  (bind _returnvalue_2 (Transformation|GetWorldLocation _turrethead_2))
  (bind _outhit (Collision|LineTraceByChannel _returnvalue_2 (+ _returnvalue_2 (* (Math|Vector|GetForwardVector (Variables|Default|GetturretHead)) (Class|KismetSystemLibrary|MakeLiteralInteger 5000))) "TraceTypeQuery1" false 0 "None" false "(R=1.000000,G=0.000000,B=0.000000,A=1.000000)" "(R=0.000000,G=1.000000,B=0.000000,A=1.000000)" 0.0))
  (if (not (Actor|ActorHasTag (.HitActor (Collision|BreakHitResult _outhit)) "Enemy"))
    (bind _returnvalue_3 (Game|SpawnActorfromClass "/Game/Turret/TurretBullet.TurretBullet_C" (Math|Transform|MakeTransform (.location _returnvalue) (.rotation _returnvalue) "0.100000,0.100000,0.100000") "Undefined" "MultiplyWithRoot" 0 0))))

(event EventBeginPlay)

(event Collision|EventActorBeginOverlap
  (params (OtherActor :type Actor%20Object%20Reference)))

(event EventTick
  (params (DeltaSeconds :type Float%20%28single-precision%29)))

(fn ConstructionScript
  (Class|InterptoMovementComponent|AddControlPointPosition (Variables|Default|GetInterpToMovement) "0, 0, 0" true)
  (Class|InterptoMovementComponent|AddControlPointPosition (Variables|Default|GetInterpToMovement) (Variables|Default|GetmoveToPos) true))