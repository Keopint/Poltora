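; BP_Platform is a crumbling platform that fades out and stops colliding after being hit, then restores itself.
; On BeginPlay it puts a dynamic M_Bright material on the Cube with its glow off.
; A hit on the Cube turns the glow up and plays a timeline that drives the opacity parameter.
; When the timeline ends, collision and glow switch off, and after a delay collision and full opacity return.
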(event OnComponentHit(Cube)
  (params (HitComponent :type Primitive%20Component%20Object%20Reference) (OtherActor :type Actor%20Object%20Reference) (OtherComp :type Primitive%20Component%20Object%20Reference) (NormalImpulse :type Vector :default "0, 0, 0") (Hit :type Hit%20Result%20Structure%20%28by%20ref%29))
  (Rendering|Material|SetScalarParameterValue (Variables|Default|GetDynamic%20Matirial) "Bright" 1e+01 :!class /Script/Engine.MaterialInstanceDynamic)
  (bind _platform_destroy (Timeline|Timeline PlayFromStart)
    (:Update
      (Rendering|Material|SetScalarParameterValue (Variables|Default|GetDynamic%20Matirial) "Opasity" _platform_destroy :!class /Script/Engine.MaterialInstanceDynamic))
    (:Finished
      (Collision|SetCollisionEnabled (Variables|Default|GetCube) "NoCollision")
      (Rendering|Material|SetScalarParameterValue (Variables|Default|GetDynamic%20Matirial) "Bright" 0.0 :!class /Script/Engine.MaterialInstanceDynamic)
      (Utilities|FlowControl|Delay 5.0)
      (Collision|SetCollisionEnabled (Variables|Default|GetCube) "QueryAndPhysics")
      (Rendering|Material|SetScalarParameterValue (Variables|Default|GetDynamic%20Matirial) "Opasity" 1.0 :!class /Script/Engine.MaterialInstanceDynamic))))

(event EventBeginPlay
  (bind _returnvalue (Rendering|Material|CreateDynamicMaterialInstance (Variables|Default|GetCube) 0 "/Game/BP_Textur_Gleb/destroyplatform/M_Bright.M_Bright" "None" :!class /Script/Engine.PrimitiveComponent))
  (bind _output_get (Variables|Default|SetDynamic%20Matirial _returnvalue))
  (Rendering|Material|SetScalarParameterValue _output_get "Bright" 0.0 :!class /Script/Engine.MaterialInstanceDynamic))

(fn ConstructionScript)