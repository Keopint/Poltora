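; BP_PatrolRoute is a patrol route actor that supplies successive waypoints along a spline.
; GetNextPointLocation returns the world-space location of the spline point at the current PatrolIndex.
; IncrementPatrolPath advances that index, using a modulo on the point count that is intended to loop the route.
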(event Custom|IncrementPatrolPath
  (bind _result (Math|Integer|IncrementInt (Variables|Default|GetPatrolIndex))
    (:%20%20
      (Variables|Default|SetPatrolIndex (Math|Integer|%(Integer) _result (Spline|GetNumberOfSplinePoints (Variables|Default|GetPatrolPath)))))))

(event EventBeginPlay)

(event Collision|EventActorBeginOverlap
  (params (OtherActor :type Actor%20Object%20Reference)))

(event EventTick
  (params (DeltaSeconds :type Float%20%28single-precision%29)))

(fn ConstructionScript)

(fn GetNextPointLocation
  (return (Spline|GetLocationatSplinePoint (Variables|Default|GetPatrolPath) (Variables|Default|GetPatrolIndex) "World")))