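; Guard robot character for AI use, exposing a patrol route, team ID and death status.
; A health component's death event triggers a one-time ragdoll, disables capsule collision and prints a debug message; damage events have no response.
; State changes are forwarded to the animation instance, while a separate event sets walk speed per state, from passive through attacking to dead.
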(event OnDamageTaken(BPC_Health_Component))

(event OnDeath(BPC_Health_Component)
  (Utilities|FlowControl|DoOnce false
    (:Completed
      (Collision|SetCollisionProfileName (Variables|Character|GetMesh) "Ragdoll" true :!class /Script/Engine.PrimitiveComponent)
      (Class|SkeletalMeshComponent|SetAllBodiesSimulatePhysics (Variables|Character|GetMesh) true)
      (Collision|SetCollisionEnabled (Variables|Collision|GetCapsuleComponent) "NoCollision")
      (Development|PrintString (Utilities|String|Append (Utilities|GetDisplayName self) "Dead")))))

(event EventBeginPlay)

(event Collision|EventActorBeginOverlap
  (params (OtherActor :type Actor%20Object%20Reference)))

(event EventTick
  (params (DeltaSeconds :type Float%20%28single-precision%29)))

(event EventChangeState
  (params (NewState :type IE_NPCState%20Enum :default "NewEnumerator0"))
  (Class|BPIAIHelper|ChangeState(Message) (Components|SkeletalMesh|GetAnimInstance (Variables|Character|GetMesh)) NewState))

(event EventModifyMovementSpeed
  (params (State :type IE_NPCState%20Enum :default "NewEnumerator0"))
  (bind _output_get (Variables|/Script/Engine.CharacterMovementComponent|SetMaxWalkSpeed (Variables|Character|GetCharacterMovement) (Utilities|Select :Index State :NewEnumerator0 1.6e+02 :NewEnumerator1 1.6e+02 :NewEnumerator2 4e+02 :NewEnumerator3 6e+02 :NewEnumerator4 0.0)))
  (Development|PrintString (Utilities|String|ToString(Float) _output_get)))

(fn ConstructionScript)

(fn GetTeamId
  (return false))

(fn IsDead
  (return (Default|IsDead (Variables|Default|GetBPC_Health_Component))))

(fn PatrolRoute
  (return (Variables|Default|GetPatrol%20Route)))