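; BPC_Health_Component is an unfinished health component for the MR-V01 character, meant to turn owner damage into damage and death notifications.
; Its damage handler broadcasts OnDamageTaken for positive damage, but the node binding it to the owner's OnTakeAnyDamage is disconnected.
; An IsDead helper tests a passed-in health value against zero, but the OnDeath branch using it is unreachable and no health is subtracted.
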(event Custom|OnTakeAnyDamage_Event
  (params (DamagedActor :type Actor%20Object%20Reference) (Damage :type Float%20%28single-precision%29) (DamageType :type Damage%20Type%20Object%20Reference) (InstigatedBy :type Controller%20Object%20Reference) (DamageCauser :type Actor%20Object%20Reference))
  (if (> Damage 0.0)
    (Default|CallOnDamageTaken)))

(event EventBeginPlay)

(event EventTick
  (params (DeltaSeconds :type Float%20%28single-precision%29)))

(fn IsDead
  (params (Health :type Float%20%28double-precision%29))
  (return (<= Health 0.0)))